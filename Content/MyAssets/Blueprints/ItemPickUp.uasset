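; Pickup item actor that a character can carry and drop, driven by its Interactable's interaction event.
; On interaction, if the character's hands are empty, it registers as the held item, disables cube collision and stores the character's held-object transform.
; Tick copies that spot's world location and rotation each frame instead of attaching.
; ItemDropped clears the spot and restores collision.
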(event `self.ReceiveBeginPlay`
  ;[0 0.9569 1] Register pick-up-event + turn off collision
  (`|ExecutionSequence`
    (:`then_1`
      (add `/Game/MyAssets/Blueprints/Interactable.interactedWithEvent` (`self.Interactable`) (delegate `PickUpItem`))
      (`KismetSystemLibrary.PrintString` "To be picked up"))))

(event `PickUpItem`
  (params (character :type "/Game/MyAssets/Blueprints/FirstPersonCharacter Object Reference"))
  ;[0 0.9569 1] Register pick-up-event + turn off collision
  (bind _holdingitem (`/Game/MyAssets/Blueprints/FirstPersonCharacter.HoldingObject` character))
  (if (not _holdingitem)
    (`/Game/MyAssets/Blueprints/FirstPersonCharacter.ToggleHoldingItem` character self)
    (`PrimitiveComponent.SetCollisionEnabled` (`self.Shape_Cube`) "NoCollision")
    (bind _heldobjectspot (`/Game/MyAssets/Blueprints/FirstPersonCharacter.HeldObjectTransform` character))
    (set `self.HeldObjectSpot` _heldobjectspot)))

(event `self.ReceiveTick`
  (params (DeltaSeconds :type "Float (single-precision)"))
  (bind _defaultsceneroot (`self.DefaultSceneRoot`))
  (bind _heldobjectspot (`self.HeldObjectSpot`))
  (bind (_returnvalue_location _returnvalue_rotation) (`KismetMathLibrary.BreakTransform` (`SceneComponent.K2_GetComponentToWorld` _heldobjectspot)))
  ;[0.5594 0.09964 0.09964] Keeps the picked-up-item following the player [every frame]
  (if (`KismetSystemLibrary.IsValid` _heldobjectspot)
    (`SceneComponent.K2_SetWorldRotation` _defaultsceneroot _returnvalue_rotation false false)
    (`SceneComponent.K2_SetWorldLocation` _defaultsceneroot _returnvalue_location false false)))

(fn `ItemDropped`
  ;[1 1 1] Set To Null + regain collision
  (set `self.HeldObjectSpot` null)
  (`PrimitiveComponent.SetCollisionEnabled` (`self.Shape_Cube`) "QueryAndPhysics"))

(fn `UserConstructionScript`)